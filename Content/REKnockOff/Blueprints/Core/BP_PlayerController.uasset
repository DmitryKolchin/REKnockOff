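; BP_PlayerController is the player controller that switches possession between the player avatar and other pawns, such as one for the inventory.
; OpenInventory possesses a given pawn with optional pause, while PossessPlayerAvatar retakes the first BP_PlayerAvatar found and unpauses.
; Possessing an avatar restores the control rotation stored on it.
; Pausing uses near-zero global time dilation rather than the engine's pause.
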(event `self.ReceivePossess`
  (params (PossessedPawn :type "Pawn Object Reference"))
  (bind _asbp_player_avatar (cast `/Game/REKnockOff/Blueprints/Core/BP_PlayerAvatar` PossessedPawn))
  (`self.SetControlRotation` (`/Game/REKnockOff/Blueprints/Core/BP_PlayerAvatar.UnpossesedControlRotation` _asbp_player_avatar)))

(event `self.ReceiveTick`
  (params (DeltaSeconds :type "Float (single-precision)")))

(fn `OpenInventory`
  (params (Pawn :type "Pawn Object Reference") (IsPaused :type Boolean))
  (`/Engine/EditorBlueprintResources/StandardMacros.IsValid` Pawn
    (:`Is Valid`
      (`self.Possess` Pawn)
      (`self.SetGamePaused` IsPaused))))

(fn `PossessPlayerAvatar`
  (bind _outactors (`GameplayStatics.GetAllActorsOfClass` "/Game/REKnockOff/Blueprints/Core/BP_PlayerAvatar.BP_PlayerAvatar_C"))
  (`self.Possess` (`|GetArrayItem` _outactors))
  (`self.SetGamePaused` false))

(fn `SetGamePaused`
  (params (IsPaused :type Boolean))
  (if IsPaused
    (`GameplayStatics.SetGlobalTimeDilation` 1e-05)
    (else
      (`GameplayStatics.SetGlobalTimeDilation` 1.0))))

(fn `UserConstructionScript`)