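; BP_Collectible is a world pickup that adds an item to the inventory and opens an inspection view of its mesh.
; Interaction passes its item class and tag to the first BP_InventoryGrid found in the level, starts inspection mode on the BP_PlayerAvatar pawn with configurable scale and rotation, then destroys the actor.
; Show and hide events toggle a widget as the interaction indicator.
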(event `/Game/REKnockOff/Blueprints/Environment/Interactables/BPI_Interactable.HideInteractionIndication`
  (`SceneComponent.SetHiddenInGame` (`self.Widget`) true false))

(event `/Game/REKnockOff/Blueprints/Environment/Interactables/BPI_Interactable.ShowInteractionIndication`
  (`SceneComponent.SetHiddenInGame` (`self.Widget`) false false))

(event `/Game/REKnockOff/Blueprints/Environment/Interactables/BPI_Interactable.Interact`
  (bind _outactors (`GameplayStatics.GetAllActorsOfClass` "/Game/REKnockOff/Blueprints/Environment/Inventory/BP_InventoryGrid.BP_InventoryGrid_C"))
  (`/Game/REKnockOff/Blueprints/Environment/Inventory/BP_InventoryGrid.AddItem` (`|GetArrayItem` _outactors) (`self.RelatedInventoryItemClass`) (`self.InventoryItemTag`))
  (bind _asbp_player_avatar (cast `/Game/REKnockOff/Blueprints/Core/BP_PlayerAvatar` (`GameplayStatics.GetPlayerPawn` 0)))
  (`/Game/REKnockOff/Blueprints/Core/BP_PlayerAvatar.StartInspectionMode` _asbp_player_avatar (`StaticMeshComponent.StaticMesh` (`self.StaticMesh`)) (`self.InspectionMeshScale`) (`self.InspectedMeshRotation`))
  (`self.K2_DestroyActor`))

(fn `UserConstructionScript`)