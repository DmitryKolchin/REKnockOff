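; Interactable swinging door that can be locked behind key items, with a widget shown or hidden as the interaction indicator.
; Interacting with a locked door checks the BP_InventoryGrid for every needed key tag, then unlocks and consumes those items without opening.
; An unlocked door swings via a timeline yaw lerp, its direction set by the player's side, and reverses when the player ends overlap.
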(event `/Game/REKnockOff/Blueprints/Environment/Interactables/BPI_Interactable.HideInteractionIndication`
  (`SceneComponent.SetHiddenInGame` (`self.Widget`) true false))

(event `/Game/REKnockOff/Blueprints/Environment/Interactables/BPI_Interactable.ShowInteractionIndication`
  (`SceneComponent.SetHiddenInGame` (`self.Widget`) false false))

(event `/Game/REKnockOff/Blueprints/Environment/Interactables/BPI_Interactable.Interact`
  (if (`self.IsLocked`)
    (if (`self.CanOpenDoor`)
      (`self.Unlock`))
    (else
      (`self.OpenDoor`))))

(event `OpenDoor`
  (set `self.OpenedDoorYawAngle` (* (`KismetMathLibrary.SignOfFloat` (`KismetMathLibrary.Dot_VectorVector` (- (`self.K2_GetActorLocation` (`GameplayStatics.GetPlayerCharacter` 0)) (`self.K2_GetActorLocation`)) (`self.GetActorForwardVector`))) 90.0))
  (`TimelineComponent.Play` (`self.DoorAnimTimeline`)))

(event `CloseDoor`
  (`TimelineComponent.Reverse` (`self.DoorAnimTimeline`)))

(event `self.ReceiveActorEndOverlap`
  (params (OtherActor :type "Actor Object Reference"))
  (if (== (`GameplayStatics.GetPlayerCharacter` 0) OtherActor)
    (`self.CloseDoor`)))

(fn `CanOpenDoor`
  (returns (CanOpen :type Boolean))
  (for _array_element (`self.NeededKeyTags`)
    (bind _outactors (`GameplayStatics.GetAllActorsOfClass` "/Game/REKnockOff/Blueprints/Environment/Inventory/BP_InventoryGrid.BP_InventoryGrid_C"))
    (bind _hasitem (`/Game/REKnockOff/Blueprints/Environment/Inventory/BP_InventoryGrid.HasItemByTag` (`|GetArrayItem` _outactors) _array_element))
    (if (not _hasitem)
      (return false)))
  (return true))

(fn `Unlock`
  (set `self.IsLocked` false)
  (for _array_element (`self.NeededKeyTags`)
    (bind _outactors (`GameplayStatics.GetAllActorsOfClass` "/Game/REKnockOff/Blueprints/Environment/Inventory/BP_InventoryGrid.BP_InventoryGrid_C"))
    (`/Game/REKnockOff/Blueprints/Environment/Inventory/BP_InventoryGrid.RemoveItemByTag` (`|GetArrayItem` _outactors) _array_element)))

(fn `UserConstructionScript`)