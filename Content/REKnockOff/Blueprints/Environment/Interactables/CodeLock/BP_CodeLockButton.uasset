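; BP_CodeLockButton is a pressable button actor for the code lock interactable.
; Press broadcasts the OnPressed dispatcher with itself as the argument, then plays a timeline that moves the Cube along its relative Y axis, scaled by PressAnimationDistance.
; Presses are ignored while the animation is playing.
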(event `Press`
  (if (not (`TimelineComponent.IsPlaying` (`self.PressedAnimTimeline`)))
    (`self.OnPressed` self)
    (bind (_direction _time) (`Timeline|PressedAnimTimeline` :!via `PlayFromStart`)
      (:`Update`
        (`SceneComponent.K2_SetRelativeLocation` (`self.Cube`) (`KismetMathLibrary.MakeVector` 0.0 (* _time (`self.PressAnimationDistance`))) false false)))))

(fn `UserConstructionScript`)