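; BP_CodeLockPawn is an interactable code lock pawn that the player possesses to operate its buttons with the mouse.
; Interacting possesses it and hides its interaction widget; possession changes toggle the cursor and code lock input mapping context.
; Press input runs a short trace under the cursor and calls Press on any BP_CodeLockButton hit.
; Quit input has BP_PlayerController repossess the player avatar.
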(event `self.HideInteractionIndication`
  (`SceneComponent.SetHiddenInGame` (`self.InteractionWidget`) true false))

(event `self.ShowInteractionIndication`
  (`SceneComponent.SetHiddenInGame` (`self.InteractionWidget`) false false))

(event `self.Interact`
  (`Controller.Possess` (`GameplayStatics.GetPlayerController` 0) self)
  (`self.HideInteractionIndication`))

(event `self.ReceiveUnpossessed`
  (params (OldController :type "Controller Object Reference"))
  (bind _asbp_player_controller (cast `/Game/REKnockOff/Blueprints/Core/BP_PlayerController` OldController))
  (set `PlayerController.bShowMouseCursor` false _asbp_player_controller)
  (`EnhancedInputSubsystemInterface.RemoveMappingContext` (pcsubsystem `EnhancedInputLocalPlayerSubsystem` _asbp_player_controller) "/Game/REKnockOff/Inputs/CodeLock/IMC_CodeLock.IMC_CodeLock" (make `ModifyContextOptions` true)))

(event `self.ReceivePossessed`
  (params (NewController :type "Controller Object Reference"))
  (bind _asbp_player_controller (cast `/Game/REKnockOff/Blueprints/Core/BP_PlayerController` NewController))
  (set `PlayerController.bShowMouseCursor` true _asbp_player_controller)
  (`EnhancedInputSubsystemInterface.AddMappingContext` (pcsubsystem `EnhancedInputLocalPlayerSubsystem` _asbp_player_controller) "/Game/REKnockOff/Inputs/CodeLock/IMC_CodeLock.IMC_CodeLock" 0 (make `ModifyContextOptions` true)))

(event `EnhancedInput|/Game/REKnockOff/Inputs/CodeLock/InputAssets/IA_Press_CodeLock`
  (params (ActionValue :type Boolean) (ElapsedSeconds :type "Float (double-precision)") (TriggeredSeconds :type "Float (double-precision)") (InputAction :type "InputAction Object Reference" :default "/Game/REKnockOff/Inputs/CodeLock/InputAssets/IA_Press_CodeLock.IA_Press_CodeLock"))
  (bind (_start _end) (`/Game/REKnockOff/Blueprints/Core/BPL_MainFunctionLibrary.GetTraceUnderCursorCoordinates` self 100.0))
  (:`Started`
    (bind _outhit (`KismetSystemLibrary.LineTraceSingle` _start _end "TraceTypeQuery1"))
    (bind _asbp_code_lock_button (cast `/Game/REKnockOff/Blueprints/Environment/Interactables/CodeLock/BP_CodeLockButton` (`.HitActor` (`GameplayStatics.BreakHitResult` _outhit))))
    (`/Game/REKnockOff/Blueprints/Environment/Interactables/CodeLock/BP_CodeLockButton.Press` _asbp_code_lock_button)))

(event `EnhancedInput|/Game/REKnockOff/Inputs/CodeLock/InputAssets/IA_Quit_CodeLock`
  (params (ActionValue :type Boolean) (ElapsedSeconds :type "Float (double-precision)") (TriggeredSeconds :type "Float (double-precision)") (InputAction :type "InputAction Object Reference" :default "/Game/REKnockOff/Inputs/CodeLock/InputAssets/IA_Quit_CodeLock.IA_Quit_CodeLock"))
  (:`Started`
    (bind _asbp_player_controller (cast `/Game/REKnockOff/Blueprints/Core/BP_PlayerController` (`self.GetController`)))
    (`/Game/REKnockOff/Blueprints/Core/BP_PlayerController.PossessPlayerAvatar` _asbp_player_controller)))

(fn `UserConstructionScript`)