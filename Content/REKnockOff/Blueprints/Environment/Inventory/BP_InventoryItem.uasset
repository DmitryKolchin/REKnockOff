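; BP_InventoryItem is a grid inventory item actor that can be picked up, moved, rotated and placed over BP_InventoryCell actors.
; While moving, Tick lerps it toward DesiredLocation, and box overlaps highlight cells as good or bad by comparing overlapped cell count to Length × Width.
; On release, it clears highlights and a timeline lerps it to the end location.
; The box is sized from item dimensions and cell spacing.
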(event `self.ReceiveBeginPlay`
  (set `self.DesiredLocation` (`self.K2_GetActorLocation`)))

(event `self.ReceiveTick`
  (params (DeltaSeconds :type "Float (single-precision)"))
  (if (`self.IsMoving`)
    (`self.K2_SetActorLocation` (`KismetMathLibrary.VLerp` (`self.K2_GetActorLocation`) (`self.DesiredLocation`) 0.1))))

(event `self.Box.OnComponentBeginOverlap`
  (params (OverlappedComponent :type "PrimitiveComponent Object Reference") (OtherActor :type "Actor Object Reference") (OtherComp :type "PrimitiveComponent Object Reference") (OtherBodyIndex :type Integer) (bFromSweep :type Boolean) (SweepResult :type "HitResult Structure (by ref)"))
  (cast `/Game/REKnockOff/Blueprints/Environment/Inventory/BP_InventoryCell` OtherActor)
  (`self.HighlightCells`))

(event `self.Box.OnComponentEndOverlap`
  (params (OverlappedComponent :type "PrimitiveComponent Object Reference") (OtherActor :type "Actor Object Reference") (OtherComp :type "PrimitiveComponent Object Reference") (OtherBodyIndex :type Integer))
  (bind _asbp_inventory_cell (cast `/Game/REKnockOff/Blueprints/Environment/Inventory/BP_InventoryCell` OtherActor))
  (`/Game/REKnockOff/Blueprints/Environment/Inventory/BP_InventoryCell.SetDefautHighlight` _asbp_inventory_cell)
  (`self.HighlightCells`))

(event `FinishMoving`
  (params (EndLocation :type "Vector Structure"))
  ;[1 1 1] Finishes the process of mouse chasing movement and places the item to the desired position
  (set `self.StartLocation` (`self.K2_GetActorLocation`))
  (set `self.DesiredLocation` (`KismetMathLibrary.MakeVector` (.x EndLocation) (.y EndLocation) (`self.DefaultHeight`)))
  (set `self.IsMoving` false)
  (`self.RemoveCellHighlight`)
  (bind (_direction _time) (`Timeline|ReturnToGridTimeline` :!via `PlayFromStart`)
    (:`Update`
      (`self.K2_SetActorLocation` (`KismetMathLibrary.VLerp` (`self.StartLocation`) (`self.DesiredLocation`) _time)))))

(event `RotateItem`
  (params (RotationAngle :type "Float (single-precision)"))
  (`self.K2_AddActorWorldRotation` (`KismetMathLibrary.MakeRotator` 0.0 0.0 RotationAngle)))

(fn `HighlightCells`
  (locals (Local_IsGoodPosition :type Boolean))
  ;[1 1 1] Highlighting tje overlapping cells in order to indicate if the item can be placed
  (if (`self.IsMoving`)
    (set `local.Local_IsGoodPosition` (>= (`KismetArrayLibrary.Array_Length` (`self.GetOverlappingActors` "/Game/REKnockOff/Blueprints/Environment/Inventory/BP_InventoryCell.BP_InventoryCell_C")) (* (`self.Width`) (`self.Length`))))
    (for _array_element (`self.GetOverlappingActors` "/Game/REKnockOff/Blueprints/Environment/Inventory/BP_InventoryCell.BP_InventoryCell_C")
      (bind _asbp_inventory_cell (cast `/Game/REKnockOff/Blueprints/Environment/Inventory/BP_InventoryCell` _array_element))
      (if (`local.Local_IsGoodPosition`)
        (`/Game/REKnockOff/Blueprints/Environment/Inventory/BP_InventoryCell.SetGoodPositionHighlight` _asbp_inventory_cell)
        (else
          (`/Game/REKnockOff/Blueprints/Environment/Inventory/BP_InventoryCell.SetBadPositionHighlight` _asbp_inventory_cell))))))

(fn `IsRotated`
  (returns (IsRotated :type Boolean))
  ;[1 1 1] Function, that checks if the item is rotated 90 or -90 degrees by yaw axis, which is needed to determine if we
  ; need to switch length and width parameters to calculate
  ; needed cell window dimensions.
  (return (`KismetMathLibrary.NearlyEqual_FloatFloat` (`KismetMathLibrary.Abs` (.yaw (`self.K2_GetActorRotation`))) 90.0 1.0)))

(fn `RemoveCellHighlight`
  (for _array_element (`self.GetOverlappingActors` "/Game/REKnockOff/Blueprints/Environment/Inventory/BP_InventoryCell.BP_InventoryCell_C")
    (bind _asbp_inventory_cell (cast `/Game/REKnockOff/Blueprints/Environment/Inventory/BP_InventoryCell` _array_element))
    (`/Game/REKnockOff/Blueprints/Environment/Inventory/BP_InventoryCell.SetDefautHighlight` _asbp_inventory_cell)))

(fn `SetCollisionBoxSize`
  (params (Local_CellSize :type "Float (double-precision)") (Local_DistanceBetweenCells :type "Float (double-precision)"))
  (locals (CollisionBoxBorderReduction :type "Float (double-precision)"))
  ;[1 1 1] Counting the collision box size based on preset item dimensions
  (`BoxComponent.SetBoxExtent` (`self.Box`) (`KismetMathLibrary.MakeVector` (/ (+ (* (- (`self.Length`) 1) (+ (`local.Local_CellSize`) (`local.Local_DistanceBetweenCells`))) (`local.Local_DistanceBetweenCells`)) 2.0) (/ (+ (* (- (`self.Width`) 1) (+ (`local.Local_CellSize`) (`local.Local_DistanceBetweenCells`))) (`local.Local_DistanceBetweenCells`)) 2.0) 100.0) true))

(fn `Start Moving`
  (`|ExecutionSequence`
    (:`then_0`
      (set `self.DesiredLocation` (`KismetMathLibrary.MakeVector` (.x (`self.K2_GetActorLocation`)) (.y (`self.K2_GetActorLocation`)) (`self.MouseFollowingHeight`)))
      (set `self.IsMoving` true)
      (`self.HighlightCells`))
    (:`then_1`
      (if (`TimelineComponent.IsPlaying` (`self.ReturnToGridTimeline`))
        (`TimelineComponent.Stop` (`self.ReturnToGridTimeline`))))))

(fn `UserConstructionScript`)