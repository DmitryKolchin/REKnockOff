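; Player pawn for a grid inventory, letting the mouse drag, rotate and place BP_InventoryItem actors.
; Left click grabs the item under the cursor, and Q/E rotate it 90 degrees while held.
; Tick traces past all items to the surface beneath and shifts the held item by the hit point's XY delta.
; On release it snaps to its overlapped cells' center if their count matches its area, otherwise to the grid's closest free window.
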(event `self.ReceiveBeginPlay`
  (set `PlayerController.bShowMouseCursor` true (`GameplayStatics.GetPlayerController` 0))
  (bind _outactors (`GameplayStatics.GetAllActorsOfClass` "/Game/REKnockOff/Blueprints/Environment/Inventory/BP_InventoryItem.BP_InventoryItem_C"))
  (set `self.IgnoredActors` _outactors)
  (bind _outactors_2 (`GameplayStatics.GetAllActorsOfClass` "/Game/REKnockOff/Blueprints/Environment/Inventory/BP_InventoryGrid.BP_InventoryGrid_C"))
  (set `self.Grid` (`|GetArrayItem` _outactors_2)))

(event `self.ReceiveTick`
  (params (DeltaSeconds :type "Float (single-precision)"))
  (bind (_start _end) (`self.GetLineTraceCoordinates`))
  (bind _moveditem (`self.MovedItem`))
  (bind _outhit (`KismetSystemLibrary.LineTraceSingle` _start _end "TraceTypeQuery1" false (`self.IgnoredActors`)))
  (bind (_bblockinghit _binitialoverlap _time _distance _location) (`GameplayStatics.BreakHitResult` _outhit))
  (if _bblockinghit
    (`|ExecutionSequence`
      (:`then_0`
        (`/Engine/EditorBlueprintResources/StandardMacros.IsValid` (`self.MovedItem`)
          (:`Is Valid`
            (set `/Game/REKnockOff/Blueprints/Environment/Inventory/BP_InventoryItem.DesiredLocation` (+ (`/Game/REKnockOff/Blueprints/Environment/Inventory/BP_InventoryItem.DesiredLocation` _moveditem) (`KismetMathLibrary.MakeVector` (.x (- _location (`self.MouseHitLocation`))) (.y (- _location (`self.MouseHitLocation`))))) _moveditem))))
      (:`then_1`
        (set `self.MouseHitLocation` _location)))))

(event `Key|LeftMouseButton`
  (params (Key :type "Key Structure"))
  (bind (_start _end) (`self.GetLineTraceCoordinates`))
  (bind _moveditem (`self.MovedItem`))
  (bind _overlappingactors (`self.GetOverlappingActors` (`self.MovedItem`) "/Game/REKnockOff/Blueprints/Environment/Inventory/BP_InventoryCell.BP_InventoryCell_C"))
  (:`Pressed`
    (bind _outhit (`KismetSystemLibrary.LineTraceSingle` _start _end "TraceTypeQuery1"))
    (bind _asbp_inventory_item (cast `/Game/REKnockOff/Blueprints/Environment/Inventory/BP_InventoryItem` (`.HitActor` (`GameplayStatics.BreakHitResult` _outhit))))
    (bind _output_get (set `self.MovedItem` _asbp_inventory_item))
    (`/Game/REKnockOff/Blueprints/Environment/Inventory/BP_InventoryItem.Start Moving` _output_get))
  (:`Released`
    (`/Engine/EditorBlueprintResources/StandardMacros.IsValid` (`self.MovedItem`)
      (:`Is Valid`
        (`/Game/REKnockOff/Blueprints/Environment/Inventory/BP_InventoryItem.FinishMoving` (`self.MovedItem`) (select `bool` (== (`KismetArrayLibrary.Array_Length` _overlappingactors) (* (`/Game/REKnockOff/Blueprints/Environment/Inventory/BP_InventoryItem.Length` _moveditem) (`/Game/REKnockOff/Blueprints/Environment/Inventory/BP_InventoryItem.Width` _moveditem))) :`false` (`.ClosestCentre` (`/Game/REKnockOff/Blueprints/Environment/Inventory/BP_InventoryGrid.GetItemClosestFreeWindowByItem` (`self.Grid`) (`self.MovedItem`))) :`true` (`/Game/REKnockOff/Blueprints/Environment/Inventory/BP_InventoryGrid.GetWindowCenter` (`self.Grid`) _overlappingactors)))
        (set `self.MovedItem` null)))))

(event `Key|Q`
  (params (Key :type "Key Structure"))
  (:`Pressed`
    (`/Engine/EditorBlueprintResources/StandardMacros.IsValid` (`self.MovedItem`)
      (:`Is Valid`
        (`/Game/REKnockOff/Blueprints/Environment/Inventory/BP_InventoryItem.RotateItem` (`self.MovedItem`) -90.0)))))

(event `Key|E`
  (params (Key :type "Key Structure"))
  (:`Pressed`
    (`/Engine/EditorBlueprintResources/StandardMacros.IsValid` (`self.MovedItem`)
      (:`Is Valid`
        (`/Game/REKnockOff/Blueprints/Environment/Inventory/BP_InventoryItem.RotateItem` (`self.MovedItem`) 90.0)))))

(fn `GetLineTraceCoordinates`
  (returns (Start :type "Vector Structure") (End :type "Vector Structure"))
  (bind (_worldlocation _worlddirection) (`PlayerController.DeprojectMousePositionToWorld` (`GameplayStatics.GetPlayerController` 0)))
  (return _worldlocation (+ _worldlocation (* _worlddirection 1000.0))))

(fn `UserConstructionScript`)