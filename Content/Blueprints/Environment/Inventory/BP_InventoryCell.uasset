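; BP_InventoryCell is a single cell of the inventory grid, drawn as a cube that shows whether a placement position is valid.
; Separate functions swap the cube's material between good position, bad position and default highlights.
; A debug black highlight function currently applies the same master material as the default.
; It has no active event logic, so highlighting relies on outside callers.
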(fn `DEBUG_SetBlackHighlight`
  (`PrimitiveComponent.SetMaterial` (`self.Cube`) 0 "/Game/Materials/Inventory/M_CellMasterMaterial.M_CellMasterMaterial"))

(fn `SetBadPositionHighlight`
  (`PrimitiveComponent.SetMaterial` (`self.Cube`) 0 "/Game/Materials/Inventory/MI_Cell_BadPosition.MI_Cell_BadPosition"))

(fn `SetDefautHighlight`
  (`PrimitiveComponent.SetMaterial` (`self.Cube`) 0 "/Game/Materials/Inventory/M_CellMasterMaterial.M_CellMasterMaterial"))

(fn `SetGoodPositionHighlight`
  (`PrimitiveComponent.SetMaterial` (`self.Cube`) 0 "/Game/Materials/Inventory/MI_Cell_GoodPosition.MI_Cell_GoodPosition"))

(fn `UserConstructionScript`)