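; Inventory grid actor that builds a Width by Length field of BP_InventoryCell child actors in its construction script and spawns items sized to that grid.
; AddItem spawns a BP_InventoryItem with a collision box matched to cell size and spacing; BeginPlay adds one hardcoded 2x4 item.
; For placement, GetClosestWindowCentre tests every cell as a window corner, keeping the in-bounds item-sized window whose centre is nearest a given location.
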(event `self.ReceiveBeginPlay`
  (`self.AddItem` "/Game/Meshes/Thor.Thor" 2 4))

(fn `AddItem`
  (params (Local_ItemMesh :type "StaticMesh Object Reference") (Local_Width :type Integer) (Local_Length :type Integer))
  (`/Engine/EditorBlueprintResources/StandardMacros.IsValid` Local_ItemMesh
    (:`Is Valid`
      (bind _returnvalue (`|SpawnActorFromClass` "/Game/Blueprints/Environment/Inventory/BP_InventoryItem.BP_InventoryItem_C" (`KismetMathLibrary.MakeTransform` (170.0 -75.0 10.0)) "Undefined" "OverrideRootScale" null (`local.Local_Width`) (`local.Local_Length`) null))
      (`/Game/Blueprints/Environment/Inventory/BP_InventoryItem.SetCollisionBoxSize` _returnvalue (`self.CellSize`) (`self.DistanceBetweenCells`)))))

(fn `DoubleToSingleIndexing`
  (params (X :type Integer) (Y :type Integer))
  (returns (Index :type Integer))
  (return (+ X (* Y (`self.Width`)))))

(fn `GenerateWindow`
  (params (Local_LeftBottomCorner :type "/Game/Blueprints/Environment/Inventory/BP_InventoryCell Object Reference") (Local_WindowWidth :type Integer) (Local_WindowLength :type Integer))
  (returns (Success :type Boolean) (Window :type "Array of /Game/Blueprints/Environment/Inventory/BP_InventoryCell Object Reference"))
  (locals (Local_Window :type "Array of /Game/Blueprints/Environment/Inventory/BP_InventoryCell Object Reference") (Local_CellIndex :type Integer :default 0) (Local_X :type Integer :default 0) (Local_Y :type Integer))
  (bind _returnvalue (`KismetArrayLibrary.Array_Find` (`self.Cells`) Local_LeftBottomCorner))
  (if (>= _returnvalue 0)
    (bind _output_get (set `local.Local_CellIndex` _returnvalue))
    (bind (_x _y) (`self.SingleToDoubleIndexing` _output_get))
    (set `local.Local_X` _x)
    (set `local.Local_Y` _y)
    (for _ (range 1 (+ (`local.Local_WindowLength`) 1))
      (if (< (`local.Local_Y`) (`self.Length`))
        (for _ (range 1 (+ (`local.Local_WindowWidth`) 1))
          (if (< (`local.Local_X`) (`self.Width`))
            (`KismetArrayLibrary.Array_Add` (`local.Local_Window`) (`|GetArrayItem` (`self.Cells`) (`self.DoubleToSingleIndexing` (`local.Local_X`) (`local.Local_Y`))))
            (`/Engine/EditorBlueprintResources/StandardMacros.IncrementInt` (`local.Local_X`))
            (else
              (return false))))
        (set `local.Local_X` (`self.SingleToDoubleIndexing` (`local.Local_CellIndex`)))
        (`/Engine/EditorBlueprintResources/StandardMacros.IncrementInt` (`local.Local_Y`))
        (else
          (return false))))
    (return true (`local.Local_Window`))
    (else
      (return false))))

(fn `Get Closest WindowCentre`
  (params (Local_Location :type "Vector Structure") (Local_Width :type Integer) (Local_Length :type Integer))
  (returns (ClosestCentre :type "Vector Structure"))
  (locals (Local_MinimalLength :type "Float (double-precision)" :default 9730175058.755287) (Local_ClosestCentre :type "Vector Structure"))
  (for _array_element (`self.Cells`)
    (bind (_success _window) (`self.GenerateWindow` _array_element (`local.Local_Width`) (`local.Local_Length`)))
    (if _success
      (bind _centrecoordinates (`self.GetWindowCentre` _window))
      (bind _returnvalue (`KismetMathLibrary.VSize` (- (`local.Local_Location`) _centrecoordinates)))
      (if (< _returnvalue (`local.Local_MinimalLength`))
        (set `local.Local_MinimalLength` _returnvalue)
        (set `local.Local_ClosestCentre` _centrecoordinates))))
  (return (`local.Local_ClosestCentre`)))

(fn `GetCellByLocation`
  (params (Local_Location :type "Vector Structure"))
  (returns (Cell :type "/Game/Blueprints/Environment/Inventory/BP_InventoryCell Object Reference"))
  (for _array_element (`self.Cells`)
    (if (== Local_Location (`self.K2_GetActorLocation` _array_element) :`ErrorTolerance` 0.1)
      (return _array_element))))

(fn `GetWindowCentre`
  (params (Cells :type "Array of Actor Object Reference"))
  (returns (CentreCoordinates :type "Vector Structure"))
  (locals (Local_TopRightCorner :type "Vector Structure") (Local_BottomLeftCorner :type "Vector Structure") (Local_CurrentCell :type "Actor Object Reference"))
  (if (`KismetArrayLibrary.Array_IsValidIndex` Cells)
    (bind _output_get (set `local.Local_TopRightCorner` (`self.K2_GetActorLocation` (`|GetArrayItem` Cells))))
    (set `local.Local_BottomLeftCorner` _output_get)
    (for _array_element Cells
      (bind _output_get_2 (set `local.Local_CurrentCell` _array_element))
      (`/Engine/EditorBlueprintResources/StandardMacros.IsValid` _output_get_2
        (:`Is Valid`
          (if (and (<= (.x (`self.K2_GetActorLocation` (`local.Local_CurrentCell`))) (.x (`local.Local_TopRightCorner`))) (<= (.y (`self.K2_GetActorLocation` (`local.Local_CurrentCell`))) (.y (`local.Local_TopRightCorner`))))
            (set `local.Local_TopRightCorner` (`self.K2_GetActorLocation` (`local.Local_CurrentCell`)))
            (elif (and (>= (.x (`self.K2_GetActorLocation` (`local.Local_CurrentCell`))) (.x (`local.Local_BottomLeftCorner`))) (>= (.y (`self.K2_GetActorLocation` (`local.Local_CurrentCell`))) (.y (`local.Local_BottomLeftCorner`))))
              (set `local.Local_BottomLeftCorner` (`self.K2_GetActorLocation` (`local.Local_CurrentCell`))))))))
    (return (/ (+ (`local.Local_TopRightCorner`) (`local.Local_BottomLeftCorner`)) 2.0))
    (else
      (return (0.0 0.0 0.0)))))

(fn `SingleToDoubleIndexing`
  (params (Index :type Integer))
  (returns (X :type Integer) (Y :type Integer))
  (return (mod Index (`self.Width`)) (/ Index (`self.Width`))))

(fn `UserConstructionScript`
  (locals (CellLocation :type "Vector Structure"))
  (bind _returnvalue (/ (`self.CellSize`) 100.0))
  (`KismetArrayLibrary.Array_Clear` (`self.Cells`))
  (for _ (range (`self.Length`))
    (for _ (range (+ (- (`self.Width`) 1 0) 1))
      (bind _returnvalue_2 (`AddComponent|NODE_AddChildActorComponent-0` :`RelativeTransform` (`KismetMathLibrary.MakeTransform` (`local.CellLocation`) (struct) (`KismetMathLibrary.MakeVector` _returnvalue _returnvalue 0.01))))
      (`ChildActorComponent.SetChildActorClass` _returnvalue_2 "/Game/Blueprints/Environment/Inventory/BP_InventoryCell.BP_InventoryCell_C")
      (bind _asbp_inventory_cell (cast `/Game/Blueprints/Environment/Inventory/BP_InventoryCell` (`ChildActorComponent.ChildActor` _returnvalue_2)))
      (`KismetArrayLibrary.Array_Add` (`self.Cells`) _asbp_inventory_cell)
      (set `local.CellLocation` (`KismetMathLibrary.MakeVector` (.x (`local.CellLocation`)) (+ (.y (`local.CellLocation`)) (+ (`self.CellSize`) (`self.DistanceBetweenCells`))))))
    (set `local.CellLocation` (`KismetMathLibrary.MakeVector` (+ (.x (`local.CellLocation`)) (+ (`self.CellSize`) (`self.DistanceBetweenCells`)))))))