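; Player pawn that lets the mouse drag and drop inventory items on a world-space inventory grid.
; Left click traces under the cursor to pick up, raise and highlight an item.
; Tick traces past all items and shifts the held item's desired XY location by the hit-point delta.
; Release snaps it to the centre of its overlapped cells if their count matches its footprint, otherwise to the grid's closest fitting window.
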(event `self.ReceiveBeginPlay`
  (set `PlayerController.bShowMouseCursor` true (`GameplayStatics.GetPlayerController` 0))
  (bind _outactors (`GameplayStatics.GetAllActorsOfClass` "/Game/Blueprints/Environment/Inventory/BP_InventoryItem.BP_InventoryItem_C"))
  (set `self.IgnoredActors` _outactors)
  (bind _outactors_2 (`GameplayStatics.GetAllActorsOfClass` "/Game/Blueprints/Environment/Inventory/BP_InventoryGrid.BP_InventoryGrid_C"))
  (set `self.Grid` (`|GetArrayItem` _outactors_2)))

(event `self.ReceiveTick`
  (params (DeltaSeconds :type "Float (single-precision)"))
  (bind (_start _end) (`self.GetLineTraceCoordinates`))
  (bind _moveditem (`self.MovedItem`))
  (bind _outhit (`KismetSystemLibrary.LineTraceSingle` _start _end "TraceTypeQuery1" false (`self.IgnoredActors`)))
  (bind (_bblockinghit _binitialoverlap _time _distance _location) (`GameplayStatics.BreakHitResult` _outhit))
  (if _bblockinghit
    (`|ExecutionSequence`
      (:`then_0`
        (`/Engine/EditorBlueprintResources/StandardMacros.IsValid` (`self.MovedItem`)
          (:`Is Valid`
            (set `/Game/Blueprints/Environment/Inventory/BP_InventoryItem.DesiredLocation` (+ (`/Game/Blueprints/Environment/Inventory/BP_InventoryItem.DesiredLocation` _moveditem) (`KismetMathLibrary.MakeVector` (.x (- _location (`self.MouseHitLocation`))) (.y (- _location (`self.MouseHitLocation`))) 0.0)) _moveditem))))
      (:`then_1`
        (set `self.MouseHitLocation` _location)))))

(event `Key|LeftMouseButton`
  (params (Key :type "Key Structure"))
  (bind (_start _end) (`self.GetLineTraceCoordinates`))
  (bind _moveditem (`self.MovedItem`))
  (bind _moveditem_2 (`self.MovedItem`))
  (bind _moveditem_3 (`self.MovedItem`))
  (bind _overlappingactors (`self.GetOverlappingActors` (`self.MovedItem`) "/Game/Blueprints/Environment/Inventory/BP_InventoryCell.BP_InventoryCell_C"))
  (:`Pressed`
    (bind _outhit (`KismetSystemLibrary.LineTraceSingle` _start _end "TraceTypeQuery1"))
    (bind _asbp_inventory_item (cast `/Game/Blueprints/Environment/Inventory/BP_InventoryItem` (`.HitActor` (`GameplayStatics.BreakHitResult` _outhit))))
    (bind _output_get (set `self.MovedItem` _asbp_inventory_item))
    (set `/Game/Blueprints/Environment/Inventory/BP_InventoryItem.IsMoving` true _output_get)
    (`/Game/Blueprints/Environment/Inventory/BP_InventoryItem.HighlightCells` _output_get)
    (set `/Game/Blueprints/Environment/Inventory/BP_InventoryItem.DesiredLocation` (`KismetMathLibrary.MakeVector` (.x (`self.K2_GetActorLocation` _output_get)) (.y (`self.K2_GetActorLocation` _output_get)) 20.0) _output_get))
  (:`Released`
    (`/Engine/EditorBlueprintResources/StandardMacros.IsValid` (`self.MovedItem`)
      (:`Is Valid`
        (`/Game/Blueprints/Environment/Inventory/BP_InventoryItem.FinishMoving` (`self.MovedItem`) (`KismetMathLibrary.MakeVector` (.x (select `bool` (== (`KismetArrayLibrary.Array_Length` _overlappingactors) (* (`/Game/Blueprints/Environment/Inventory/BP_InventoryItem.Length` _moveditem) (`/Game/Blueprints/Environment/Inventory/BP_InventoryItem.Width` _moveditem))) :`false` (`/Game/Blueprints/Environment/Inventory/BP_InventoryGrid.Get Closest WindowCentre` (`self.Grid`) (`self.K2_GetActorLocation` (`self.MovedItem`)) (`/Game/Blueprints/Environment/Inventory/BP_InventoryItem.Width` _moveditem_3) (`/Game/Blueprints/Environment/Inventory/BP_InventoryItem.Length` _moveditem_3)) :`true` (`/Game/Blueprints/Environment/Inventory/BP_InventoryGrid.GetWindowCentre` (`self.Grid`) _overlappingactors))) (.y (select `bool` (== (`KismetArrayLibrary.Array_Length` _overlappingactors) (* (`/Game/Blueprints/Environment/Inventory/BP_InventoryItem.Length` _moveditem) (`/Game/Blueprints/Environment/Inventory/BP_InventoryItem.Width` _moveditem))) :`false` (`/Game/Blueprints/Environment/Inventory/BP_InventoryGrid.Get Closest WindowCentre` (`self.Grid`) (`self.K2_GetActorLocation` (`self.MovedItem`)) (`/Game/Blueprints/Environment/Inventory/BP_InventoryItem.Width` _moveditem_3) (`/Game/Blueprints/Environment/Inventory/BP_InventoryItem.Length` _moveditem_3)) :`true` (`/Game/Blueprints/Environment/Inventory/BP_InventoryGrid.GetWindowCentre` (`self.Grid`) _overlappingactors))) (- (.z (`self.K2_GetActorLocation` (`self.MovedItem`))) 10.0)))
        (set `/Game/Blueprints/Environment/Inventory/BP_InventoryItem.IsMoving` false _moveditem_2)
        (`/Game/Blueprints/Environment/Inventory/BP_InventoryItem.RemoveCellHighlight` _moveditem_2)
        (set `self.MovedItem` null)))))

(fn `GetLineTraceCoordinates`
  (returns (Start :type "Vector Structure") (End :type "Vector Structure"))
  (bind (_worldlocation _worlddirection) (`PlayerController.DeprojectMousePositionToWorld` (`GameplayStatics.GetPlayerController` 0)))
  (return _worldlocation (+ _worldlocation (* _worlddirection 1000.0))))

(fn `UserConstructionScript`)