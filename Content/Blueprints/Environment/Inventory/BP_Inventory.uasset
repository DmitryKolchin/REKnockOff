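; BP_Inventory is an inventory actor that lays out a flat grid of BP_InventoryCell actors.
; The Construction Script clears the Cells array, then nested Length and Width loops add a child actor component per cell, scaled from CellSize and offset by DistanceBetweenCells.
; Each spawned cell is cast and stored in Cells.
; The event graph holds no active logic.
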(fn `UserConstructionScript`
  (locals (CellLocation :type "Vector Structure"))
  (bind _returnvalue (/ (`self.CellSize`) 100.0))
  (`KismetArrayLibrary.Array_Clear` (`self.Cells`))
  (for _ (range (`self.Length`))
    (for _ (range (+ (- (`self.Width`) 1 0) 1))
      (bind _returnvalue_2 (`AddComponent|NODE_AddChildActorComponent-0` :`RelativeTransform` (`KismetMathLibrary.MakeTransform` (`local.CellLocation`) (struct) (`KismetMathLibrary.MakeVector` _returnvalue _returnvalue 0.01))))
      (`ChildActorComponent.SetChildActorClass` _returnvalue_2 "/Game/Blueprints/Environment/Inventory/BP_InventoryCell.BP_InventoryCell_C")
      (bind _asbp_inventory_cell (cast `/Game/Blueprints/Environment/Inventory/BP_InventoryCell` (`ChildActorComponent.ChildActor` _returnvalue_2)))
      (`KismetArrayLibrary.Array_Add` (`self.Cells`) _asbp_inventory_cell)
      (set `local.CellLocation` (`KismetMathLibrary.MakeVector` (+ (.x (`local.CellLocation`)) (+ (`self.CellSize`) (`self.DistanceBetweenCells`))) (.y (`local.CellLocation`)))))
    (set `local.CellLocation` (`KismetMathLibrary.MakeVector` 0.0 (+ (.y (`local.CellLocation`)) (+ (`self.CellSize`) (`self.DistanceBetweenCells`)))))))