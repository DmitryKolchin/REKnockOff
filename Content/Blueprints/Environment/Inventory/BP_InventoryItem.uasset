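; BP_InventoryItem is a grid-based inventory item with a box collision component sized from its Length and Width in cells.
; SetCollisionBoxSize takes cell size and spacing, spans one step fewer than each dimension's cell count, subtracts a border reduction, and halves the result for the extents.
; The box height is fixed, and the event graph and construction script hold no logic.
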(fn `SetCollisionBoxSize`
  (params (Local_CellSize :type "Float (double-precision)") (Local_DistanceBetweenCells :type "Float (double-precision)"))
  (locals (CollisionBoxBorderReduction :type "Float (double-precision)"))
  (`BoxComponent.SetBoxExtent` (`self.Box`) (`KismetMathLibrary.MakeVector` (/ (- (* (- (`self.Length`) 1) (+ (`local.Local_CellSize`) (`local.Local_DistanceBetweenCells`))) (`local.CollisionBoxBorderReduction`)) 2.0) (/ (- (* (- (`self.Width`) 1) (+ (`local.Local_CellSize`) (`local.Local_DistanceBetweenCells`))) (`local.CollisionBoxBorderReduction`)) 2.0) 100.0) true))

(fn `UserConstructionScript`)